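; Base character Blueprint for a team deathmatch (TDM) player, adding a team label and key-driven weapon attachments.
; BeginPlay starts a looping half-second timer that polls the TDM player state's team and sets the TextRender to red Alpha or blue Bravo.
; The G and T keys spawn muzzle and holo attachments, respectively, and add them to the weapon in hand if it is valid.
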(event `Key|G`
  (params (Key :type "Key Structure"))
  (bind _weaponinhand (`self.WeaponInHand`))
  (:`Pressed`
    (`/Engine/EditorBlueprintResources/StandardMacros.IsValid` _weaponinhand
      (:`Is Valid`
        (bind _returnvalue (`|SpawnActorFromClass` "/Game/BlueprintClasses/game/Weapon/BP_TDMAttachment_Muzzle.BP_TDMAttachment_Muzzle_C" (`KismetMathLibrary.MakeTransform` (0.0 0.0 0.0)) "Undefined" "OverrideRootScale" self null))
        (`TDMWeaponBase.AddAttachment` _weaponinhand _returnvalue)))))

(event `Key|T`
  (params (Key :type "Key Structure"))
  (bind _weaponinhand (`self.WeaponInHand`))
  (:`Pressed`
    (`/Engine/EditorBlueprintResources/StandardMacros.IsValid` _weaponinhand
      (:`Is Valid`
        (bind _returnvalue (`|SpawnActorFromClass` "/Game/BlueprintClasses/game/Weapon/BP_TDMAttachment_Holo.BP_TDMAttachment_Holo_C" (`KismetMathLibrary.MakeTransform` (0.0 0.0 0.0)) "Undefined" "OverrideRootScale" self null))
        (`TDMWeaponBase.AddAttachment` _weaponinhand _returnvalue)))))

(event `self.ReceiveBeginPlay`
  (`KismetSystemLibrary.K2_SetTimer` null "SetTextRender" 0.5 true))

(fn `SetTextRender`
  (bind _textrender (`self.TextRender`))
  (bind _textrender_2 (`self.TextRender`))
  (bind _asbp_tdmplayer_state (cast `/Game/BlueprintClasses/Player/BP_TDMPlayerState` (`self.PlayerState`)))
  (switch `ETeam` (`TDMPlayerState.GetTeam` _asbp_tdmplayer_state)
    (:`Alpha`
      ;[1 1 1] Alpha Team Text
      (`TextRenderComponent.K2_SetText` _textrender_2 "Alpha")
      (`TextRenderComponent.SetTextRenderColor` _textrender_2 (make `Color` 0 0 255 255)))
    (:`Bravo`
      ;[1 1 1] Bravo Team Text
      (`TextRenderComponent.K2_SetText` _textrender "Bravo")
      (`TextRenderComponent.SetTextRenderColor` _textrender (make `Color` 255 0 0 255)))))

(fn `UserConstructionScript`)